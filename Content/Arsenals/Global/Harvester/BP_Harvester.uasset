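; Harvester pawn that binds itself to an AI controller and to the nearest Tiberium refinery when play begins.
; BeginPlay spawns a BP_HarvesterController, possesses itself with it and sets the controller's Harvester reference.
; It searches all BP_TiberiumRefinery actors for the closest, writes that to the OriginalRefinery blackboard key and caches it as MOwningRefinery.
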(event `self.ReceiveBeginPlay`
  (bind _returnvalue (`|SpawnActorFromClass` "/Game/AI/Harvester/BP_HarvesterController.BP_HarvesterController_C" (`self.GetTransform`) "Undefined" "OverrideRootScale" null null))
  (`Controller.Possess` _returnvalue self)
  (set `/Game/AI/Harvester/BP_HarvesterController.Harvester` self _returnvalue)
  (bind _outactors (`GameplayStatics.GetAllActorsOfClass` "/Game/Arsenals/Global/BP_TiberiumRefinery.BP_TiberiumRefinery_C"))
  (bind _closestactor (`/Game/AI/Harvester/Helpers.GetClosestObjectFromOriginToArray` _outactors self))
  (`BlackboardComponent.SetValueAsObject` (`AIBlueprintHelperLibrary.GetBlackboard` _returnvalue) "OriginalRefinery" _closestactor)
  (bind _asbp_tiberium_refinery (cast `/Game/Arsenals/Global/BP_TiberiumRefinery` _closestactor))
  (set `self.m_OwningRefinery` _asbp_tiberium_refinery))

(fn `UserConstructionScript`)