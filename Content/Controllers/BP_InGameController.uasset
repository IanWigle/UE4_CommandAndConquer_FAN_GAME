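; In-game player controller for what appears to be an RTS, handling the attack cursor and building spawning.
; BeginPlay creates an attack cursor widget and sets it as the Crosshairs cursor.
; While units are selected, Tick traces under the cursor and compares a hit unit's team to the player's, though both branches reapply that same cursor.
; SpawnBuildingFromID spawns a building, currently only Powerplant, and records it on the player character.
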(event `self.ReceiveBeginPlay`
  (bind _returnvalue (`|CreateWidget` "/Game/Cursors/AttackCursorWidget.AttackCursorWidget_C"))
  (set `self.AttackCusor` _returnvalue)
  (`self.SetMouseCursorWidget` "Crosshairs" (`self.AttackCusor`) :!label _label))

(event `self.ReceiveTick`
  (params (DeltaSeconds :type "Float (single-precision)"))
  (bind (_hitresult _returnvalue) (`self.GetHitResultUnderCursorByChannel` "TraceTypeQuery3" false))
  (bind _asbp_player_character (cast `/Game/BP_PlayerCharacter` (`self.K2_GetPawn`)))
  (bind _returnvalue_2 (`PlayerCharacter.AreUnitsSelected` _asbp_player_character))
  (if (and _returnvalue_2 _returnvalue)
    (bind _asunit (cast `Unit` (`.HitActor` (`GameplayStatics.BreakHitResult` _hitresult))))
    (if (`|EnumEquality` (`Unit.m_Team` _asunit) (`PlayerCharacter.m_PlayerTeam` _asbp_player_character))
      (goto _label)
      (else
        (goto _label)))))

(fn `SpawnBuildingFromID`
  (params (ID :type "BuildingID Enum" :default "VE_NA") (SpawnPosition :type "Vector Structure"))
  (bind _asplayer_character (cast `PlayerCharacter` (`self.K2_GetPawn`)))
  (switch `BuildingID` ID
    (:`VE_Powerplant`
      (bind _returnvalue (`|SpawnActorFromClass` "/Game/Arsenals/Global/BP_Powerplant.BP_Powerplant_C" (`KismetMathLibrary.MakeTransform` SpawnPosition) "AdjustIfPossibleButAlwaysSpawn" "OverrideRootScale" _asplayer_character null))
      (`KismetArrayLibrary.Array_Add` (`PlayerCharacter.m_PlayerBuildings` _asplayer_character) _returnvalue))))

(fn `UserConstructionScript`)