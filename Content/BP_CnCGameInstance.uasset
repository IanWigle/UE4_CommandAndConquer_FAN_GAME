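; Game instance that owns audio volume settings and creates the graphics and sound menu widgets at startup.
; Init sets the base GameSoundMix after a short delay, seeds the stored volume struct and creates both menus.
; SetVolume applies clamped per-channel sound class overrides and records each value.
; Master, Music and EVA also directly adjust the player character's music or EVA voice components, while ChangeVolume only overrides the master class.
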(event `self.ReceiveInit`
  (`KismetSystemLibrary.Delay` 0.2)
  (`GameplayStatics.SetBaseSoundMix` "/Game/Audio/GameSoundMix.GameSoundMix")
  (set `self.VolumeFloatValues` (make `/Game/Audio/SoundVolume` 1.0))
  (bind _returnvalue (`|CreateWidget` "/Game/Menus/GraphicMenu.GraphicMenu_C"))
  (set `self.GraphicsMenu` _returnvalue)
  (bind _returnvalue_2 (`|CreateWidget` "/Game/Menus/SoundMenu.SoundMenu_C"))
  (set `self.SoundMenu` _returnvalue_2))

(event `ChangeVolume`
  (params (MasterVolume :type "Float (double-precision)"))
  (bind _output_get (set `self.m_MasterAudioVolume` MasterVolume))
  (`GameplayStatics.SetSoundMixClassOverride` "/Game/Audio/GameSoundMix.GameSoundMix" "/Game/Audio/MasterSoundClass.MasterSoundClass" (`KismetMathLibrary.FClamp` _output_get 0.01)))

(fn `SetVolume`
  (params (Volume :type "Float (double-precision)") (Channel :type "/Game/Audio/SoundChannelsEnum Enum" :default "NewEnumerator0"))
  (bind _returnvalue (`KismetMathLibrary.FClamp` Volume 0.01))
  (switch `/Game/Audio/SoundChannelsEnum` Channel
    (:`NewEnumerator0`
      (`GameplayStatics.SetSoundMixClassOverride` "/Game/Audio/GameSoundMix.GameSoundMix" "/Game/Audio/MasterSoundClass.MasterSoundClass" _returnvalue)
      (setmembers `/Game/Audio/SoundVolume` :`StructRef` (`self.VolumeFloatValues`) :`MasterVolume` _returnvalue)
      (bind _asbp_player_character (cast `/Game/BP_PlayerCharacter` (`GameplayStatics.GetPlayerPawn` 0)))
      (`AudioComponent.AdjustVolume` (`MusicPlayerComponent.m_AudioComponent` (`PlayerCharacter.m_MusicPlayer` _asbp_player_character)) 0.0 _returnvalue)
      (`AudioComponent.AdjustVolume` (`PlayerCharacter.m_EVAVoiceComponent` _asbp_player_character) 0.0 _returnvalue))
    (:`NewEnumerator1`
      (`GameplayStatics.SetSoundMixClassOverride` "/Game/Audio/GameSoundMix.GameSoundMix" "/Game/Audio/VoiceSoundClass.VoiceSoundClass" _returnvalue)
      (setmembers `/Game/Audio/SoundVolume` :`StructRef` (`self.VolumeFloatValues`) :`VoiceVolume` _returnvalue))
    (:`NewEnumerator2`
      (`GameplayStatics.SetSoundMixClassOverride` "/Game/Audio/GameSoundMix.GameSoundMix" "/Game/Audio/MusicSoundClass.MusicSoundClass" _returnvalue)
      (setmembers `/Game/Audio/SoundVolume` :`StructRef` (`self.VolumeFloatValues`) :`MusicVolume` _returnvalue)
      (bind _asbp_player_character_2 (cast `/Game/BP_PlayerCharacter` (`GameplayStatics.GetPlayerPawn` 0)))
      (`AudioComponent.AdjustVolume` (`MusicPlayerComponent.m_AudioComponent` (`PlayerCharacter.m_MusicPlayer` _asbp_player_character_2)) 0.0 _returnvalue))
    (:`NewEnumerator3`
      (`GameplayStatics.SetSoundMixClassOverride` "/Game/Audio/GameSoundMix.GameSoundMix" "/Game/Audio/EffectsSoundClass.EffectsSoundClass" _returnvalue)
      (setmembers `/Game/Audio/SoundVolume` :`StructRef` (`self.VolumeFloatValues`) :`EffectsVolume` _returnvalue))
    (:`NewEnumerator4`
      (`GameplayStatics.SetSoundMixClassOverride` "/Game/Audio/GameSoundMix.GameSoundMix" "/Game/Audio/EVASoundClass.EVASoundClass" _returnvalue)
      (setmembers `/Game/Audio/SoundVolume` :`StructRef` (`self.VolumeFloatValues`) :`EVAVolume` _returnvalue)
      (bind _asbp_player_character_3 (cast `/Game/BP_PlayerCharacter` (`GameplayStatics.GetPlayerPawn` 0)))
      (`AudioComponent.AdjustVolume` (`PlayerCharacter.m_EVAVoiceComponent` _asbp_player_character_3) 0.0 _returnvalue))))