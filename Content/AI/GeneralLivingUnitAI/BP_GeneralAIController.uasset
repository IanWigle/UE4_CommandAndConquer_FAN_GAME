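; AI controller for living units that runs a shared general behavior tree on the pawn it controls.
; On BeginPlay it starts the tree, casts the controlled pawn to LivingUnit and stores it as the owning unit.
; It then seeds the blackboard with that unit's attack cooldown and attack behavior enum, so the one tree receives per-unit combat settings.
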(event `self.ReceiveBeginPlay`
  (bind _returnvalue (`AIBlueprintHelperLibrary.GetBlackboard` null))
  (`self.RunBehaviorTree` "/Game/AI/GeneralLivingUnitAI/GeneralBehaviorTree.GeneralBehaviorTree")
  (bind _asliving_unit (cast `LivingUnit` (`self.K2_GetPawn`)))
  (set `self.OwningUnit` _asliving_unit)
  (`BlackboardComponent.SetValueAsFloat` _returnvalue "AttackCooldown" (`LivingUnit.m_AttackCooldown` _asliving_unit))
  (`BlackboardComponent.SetValueAsEnum` _returnvalue "UnitAttackBehavior" (`LivingUnit.m_UnitAttackBehavior` _asliving_unit)))

(fn `UserConstructionScript`)